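; Mover movement mode transition that takes the character out of sliding and back to Walking.
; Evaluate switches to Walking when the CharacterMoverComponent is no longer crouching or the proposed horizontal speed drops to a low threshold.
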(fn Evaluate
  (params (Params :type Simulation%20Tick%20Params%20Structure%20%28by%20ref%29))
  (bind (_simcontext _movingcomps _simblackboard _startstate _timestep _proposedmove) (Utilities|Struct|BreakSimulationTickParams Params))
  (if (or (not (Class|CharacterMoverComponent|IsCrouching (.AsCharacter%20Mover%20Component (Utilities|Casting|CastToCharacterMoverComponent (.MoverComponent (Utilities|Struct|BreakMovingComponentSet _movingcomps)))))) (<= (Math|Vector|VectorLengthXY (.LinearVelocity (Utilities|Struct|BreakProposedMove _proposedmove))) 2e+02))
    (return (Utilities|Struct|MakeTransitionEvalResult "Walking"))))